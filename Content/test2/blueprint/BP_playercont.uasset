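; BP_playercont is a player controller that sets Game and UI input on BeginPlay, focusing the HUD widget from BP_gamemodedefault and keeping the cursor visible during capture.
; The primary action input sets a Lmbisdown flag while held.
; Drag-to-look logic for spring arm pitch and character yaw checks that flag but is disconnected, and the MouseX and MouseY events are empty.
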(event `self.ReceiveBeginPlay`
  (bind _asbp_gamemodedefault (cast `/Game/test2/blueprint/gamemode/BP_gamemodedefault` (`GameplayStatics.GetGameMode`)))
  (`WidgetBlueprintLibrary.SetInputMode_GameAndUIEx` (`GameplayStatics.GetPlayerController` 0) (`/Game/test2/blueprint/gamemode/BP_gamemodedefault.hud` _asbp_gamemodedefault) "DoNotLock" false))

(event `InputAxisKey|MouseY`
  (params (AxisValue :type "Float (single-precision)")))

(event `InputAxisKey|MouseX`
  (params (AxisValue :type "Float (single-precision)")))

(event `InputAction|primary action`
  (params (Key :type "Key Structure"))
  (:`Pressed`
    (set `self.lmbisdown` true))
  (:`Released`
    (set `self.lmbisdown` false)))

(fn `UserConstructionScript`)