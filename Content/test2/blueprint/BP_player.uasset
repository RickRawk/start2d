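; BP_player is a player character Blueprint that handles movement, jumping and a starting health readout.
; The axisy input stores its value in Deltamove.X, and Tick applies Deltamove as forward/right movement input when non-zero; axisX is unwired.
; A jump pressed at jump count one clears horizontal velocity and grants full air control; other jumps use reduced air control.
; BeginPlay sets Maxheatlth from Starting and prints it.
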(event `self.ReceiveBeginPlay`
  (bind _output_get (set `self.maxheatlth` (`self.starting`)))
  (`KismetSystemLibrary.PrintString` (`KismetStringLibrary.Concat_StrStr` (`KismetStringLibrary.Conv_IntToString` _output_get) "Health")))

(event `InputAction|jump`
  (params (Key :type "Key Structure"))
  (bind (_returnvalue_x _returnvalue_y _returnvalue_z) (`KismetMathLibrary.BreakVector` (`self.GetVelocity`)))
  (bind _charactermovement (`self.CharacterMovement`))
  (:`Pressed`
    (if (== (`self.JumpCurrentCount`) 1)
      (set `CharacterMovementComponent.AirControl` 1.0 _charactermovement)
      (set `MovementComponent.Velocity` (`KismetMathLibrary.MakeVector` 0.0 0.0 _returnvalue_z) _charactermovement)
      (else
        (set `CharacterMovementComponent.AirControl` 0.25 _charactermovement)))
    (`self.Jump`)))

(event `self.ReceiveTick`
  (params (DeltaSeconds :type "Float (single-precision)"))
  (`self.domovement`))

(event `InputAxis|axisX`
  (params (AxisValue :type "Float (single-precision)")))

(event `InputAxis|axisy`
  (params (AxisValue :type "Float (single-precision)"))
  (`self.setdeltamove` (`KismetMathLibrary.MakeVector` AxisValue)))

(fn `checkifmoving`
  (returns (result :type Boolean))
  (bind (_deltamove_x _deltamove_y _deltamove_z) (`KismetMathLibrary.BreakVector` (`self.deltamove`)))
  (return (or (!= _deltamove_x 0.0) (!= _deltamove_y 0.0) (!= _deltamove_z 0.0))))

(fn `domovement`
  (bind (_deltamove_x _deltamove_y) (`KismetMathLibrary.BreakVector` (`self.deltamove`)))
  (if (`self.checkifmoving`)
    (`self.AddMovementInput` (`self.GetActorForwardVector`) _deltamove_x)
    (`self.AddMovementInput` (`self.GetActorRightVector`) _deltamove_y)))

(fn `setdeltamove`
  (params (newdeltamove :type "Vector Structure") (debug :type Boolean))
  (bind _output_get (set `self.deltamove` newdeltamove))
  (if debug
    (`KismetSystemLibrary.PrintString` (`KismetStringLibrary.Concat_StrStr` "current delta move" (`KismetStringLibrary.Conv_VectorToString` _output_get)))))

(fn `UserConstructionScript`)